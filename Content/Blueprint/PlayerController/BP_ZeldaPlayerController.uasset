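; Player controller for the Zelda character that owns the health bar HUD and provides keys to change health.
; On possess it creates WBP_HealthBar and adds it to the top-left of the viewport.
; Q and T increase or decrease current and max health through the character's InventoryComponent.
; Tick re-assigns the component's OnHealthChanged delegate every frame, and that event refreshes the health bar.
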(event Custom|OnHealthChanged_이벤트
  (Default|UpdateHealthBar (Variables|Default|GetHealthBar%20Widget)))

(event EventBeginPlay)

(event EventTick
  (params (DeltaSeconds :type Float%20%28single-precision%29))
  (bind _asbp_zelda (Utilities|Casting|CastToBP_Zelda (Game|GetPlayerCharacter 0)))
  (EventDispatchers|AssignOnHealthChanged (Variables|/Script/InventoryUI.Zelda|GetInventoryComponent _asbp_zelda) (delegate Custom|OnHealthChanged_이벤트)))

(event EventPossess
  (params (PossessedPawn :type Pawn%20Object%20Reference))
  (bind _returnvalue (UserInterface|CreateWidget "/Game/Blueprint/WBP/WBP_HealthBar.WBP_HealthBar_C" self))
  (Variables|Default|SetHealthBar%20Widget _returnvalue)
  (Class|UserWidget|SetPositioninViewport _returnvalue "(X=10.000000,Y=10.000000)" true)
  (UserInterface|Viewport|AddtoViewport _returnvalue 0))

(event Input|KeyboardEvents|Q
  (params (Key :type Key%20Structure :default "None"))
  (:Pressed
    (bind _asbp_zelda (Utilities|Casting|CastToBP_Zelda (Game|GetPlayerCharacter 0)))
    (Class|InventoryComponent|IncreaseHealth (Variables|/Script/InventoryUI.Zelda|GetInventoryComponent _asbp_zelda) 5.0 1e+01)))

(event Input|KeyboardEvents|T
  (params (Key :type Key%20Structure :default "None"))
  (:Pressed
    (bind _asbp_zelda (Utilities|Casting|CastToBP_Zelda (Game|GetPlayerCharacter 0)))
    (Class|InventoryComponent|DecreaseHealth (Variables|/Script/InventoryUI.Zelda|GetInventoryComponent _asbp_zelda) 5.0 1e+01)))

(fn ConstructionScript)